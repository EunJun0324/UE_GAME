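; Wizard AI enemy that fights with two spell weapons, Fire Ball and Warp.
; On BeginPlay it spawns both weapon actors with itself as owner and stores references to them.
; Equip_Weapon switches to the requested spell only while the state is idle, calling begin and end equip back to back when the weapon change succeeds.
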(event Custom|Equip_Weapon
  (params (InWeaponType :type EWeaponType%20Enum :default "NewEnumerator0"))
  (switch Utilities|FlowControl|Switch|SwitchonEWeaponType InWeaponType
    (:NewEnumerator4
      (bind _result (CallFunction|IsStateIdle))
      (if _result
        (bind _result_2 (CallFunction|WeaponChange (Variables|Default|GetFireBall)))
        (if _result_2
          (CallFunction|WeaponBeginEquip)
          (CallFunction|WeaponEndEquip))))
    (:NewEnumerator6
      (bind _result_3 (CallFunction|IsStateIdle))
      (if _result_3
        (bind _result_4 (CallFunction|WeaponChange (Variables|Default|GetWarp)))
        (if _result_4
          (CallFunction|WeaponBeginEquip)
          (CallFunction|WeaponEndEquip))))))

(event EventBeginPlay
  (|CallParentFunction)
  (bind _returnvalue (Game|SpawnActorfromClass "/Game/Weapons/FireBall/BP_FireBall.BP_FireBall_C" (Math|Transform|MakeTransform "0, 0, 0") "Undefined" self 0))
  (Variables|Default|SetFireBall _returnvalue)
  (bind _returnvalue_2 (Game|SpawnActorfromClass "/Game/Weapons/BP_Warp.BP_Warp_C" (Math|Transform|MakeTransform "0, 0, 0") "Undefined" self 0))
  (Variables|Default|SetWarp _returnvalue_2))

(fn ConstructionScript
  (|CallParentFunction))