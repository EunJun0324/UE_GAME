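; AI controller for melee enemies that runs the possessed BP_AI pawn's behavior tree and tracks the player by sight.
; On possession it starts the tree assigned on the pawn, if one is valid.
; Perception updates scan currently seen actors for a BP_Player, write it to the "Player" blackboard key and break the loop.
; If no player is found, it clears that key.
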(event OnPerceptionUpdated(AIPerception)
  (params (UpdatedActors :type Array%20of%20Actor%20Object%20References))
  (Variables|Default|SetFindPlayer false)
  (bind _array_element (Utilities|Array|ForEachLoopwithBreak (Class|AIPerceptionComponent|GetCurrentlyPerceivedActors (Variables|Default|GetAIPerception) "/Script/AIModule.AISense_Sight"))
    (:LoopBody
      (bind _asbp_player (Utilities|Casting|CastToBP_Player _array_element))
      (AI|Components|Blackboard|SetValueasObject (AI|GetBlackboard 0) (Utilities|Name|MakeLiteralName "Player") _asbp_player)
      (Variables|Default|SetFindPlayer true)
      (CallFunction|PerceptionUpdateBreak))
    (:Completed
      (if (not (Variables|Default|GetFindPlayer))
        (AI|Components|Blackboard|SetValueasObject (AI|GetBlackboard 0) (Utilities|Name|MakeLiteralName "Player") 0)))))

(event Custom|PerceptionUpdate_Break
  (Utilities|Array|ForEachLoopwithBreak (Class|AIPerceptionComponent|GetCurrentlyPerceivedActors (Variables|Default|GetAIPerception) "/Script/AIModule.AISense_Sight")) ; enters at Break
)

(event EventPossess
  (params (PossessedPawn :type Pawn%20Object%20Reference))
  (bind _asbp_ai (Utilities|Casting|CastToBP_AI PossessedPawn))
  (bind _output_get (Variables|Default|SetAIPawn _asbp_ai))
  (bind _behaviortree (Variables|/Game/Enemies/BP_AI.BP_AI_C|GetBehaviorTree _output_get)
    (:then
      (AI|RunBehaviorTree _behaviortree))
    (:else)))

(fn ConstructionScript)