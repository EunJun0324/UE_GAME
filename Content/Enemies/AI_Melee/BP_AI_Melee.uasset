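; BP_AI_Melee is a melee AI enemy that arms itself with a two-handed weapon at the start of play.
; After the parent BeginPlay, it spawns an owned BP_Melee_TwoHand and stores it as TwoHand.
; If its state is idle and WeaponChange to that weapon succeeds, it plays the equip montage using its equip data.
; The construction script only calls the parent.
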(event EventBeginPlay
  (|CallParentFunction)
  (bind _returnvalue (Game|SpawnActorfromClass "/Game/Weapons/Melee/BP_Melee_TwoHand.BP_Melee_TwoHand_C" (Math|Transform|MakeTransform "0, 0, 0") "Undefined" self 0))
  (Variables|Default|SetTwoHand _returnvalue)
  (bind _result (CallFunction|IsStateIdle))
  (if _result
    (bind _result_2 (CallFunction|WeaponChange (Variables|Default|GetTwoHand)))
    (if _result_2
      (CallFunction|PlayEquipMontage self "NewEnumerator3" (Variables|Default|GetEquipDatas)))))

(fn ConstructionScript
  (|CallParentFunction))