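; BP_Sound3D is an actor that toggles a positional sound through a Box trigger, apparently to demonstrate 3D audio.
; Ending an overlap spawns the dirt-step cue at the actor's location and stores it, while beginning an overlap destroys the stored sound.
; While that sound is valid, Tick draws horizontal green inner and red outer debug circles around the actor, likely visualizing attenuation range.
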(event OnComponentEndOverlap(Box)
  (params (OverlappedComponent :type Primitive%20Component%20Object%20Reference) (OtherActor :type Actor%20Object%20Reference) (OtherComp :type Primitive%20Component%20Object%20Reference) (OtherBodyIndex :type Integer))
  (bind _returnvalue (Audio|SpawnSoundatLocation "/Game/Sounds/S_Stepdirt_Cue.S_Stepdirt_Cue" (Transformation|GetActorLocation) "0, 0, 0" 1.0 1.0 0.0 0 0))
  (Variables|Default|SetSound _returnvalue))

(event OnComponentBeginOverlap(Box)
  (params (OverlappedComponent :type Primitive%20Component%20Object%20Reference) (OtherActor :type Actor%20Object%20Reference) (OtherComp :type Primitive%20Component%20Object%20Reference) (OtherBodyIndex :type Integer) (bFromSweep :type Boolean) (SweepResult :type Hit%20Result%20Structure%20%28by%20ref%29))
  (bind _sound (Variables|Default|GetSound)
    (:then
      (Components|DestroyComponent _sound))
    (:else)))

(event EventTick
  (params (DeltaSeconds :type Float%20%28single-precision%29))
  (Variables|Default|GetSound
    (:then
      (Rendering|Debug|DrawDebugCircle (Transformation|GetActorLocation) 5e+02 100 "(R=0.000000,G=1.000000,B=0.000000,A=1.000000)" 0.0 0.0 "1.000000,0.000000,0.000000" "0.000000,1.000000,0.000000")
      (Rendering|Debug|DrawDebugCircle (Transformation|GetActorLocation) 2e+03 100 "(R=1.000000,G=0.000000,B=0.000000,A=1.000000)" 0.0 0.0 "1.000000,0.000000,0.000000" "0.000000,1.000000,0.000000"))
    (:else)))

(fn ConstructionScript)