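; Melee weapon Blueprint that runs indexed combo attacks and deals damage to actors its shapes overlap.
; An attack starts only when the owner's IState is idle; input during the combo window queues the next action, which BeginDoAction plays.
; EndDoAction resets the index and returns the owner to idle.
; Shape collision starts disabled, with On/Off toggles, and overlaps send the current action's damage, ignoring owner and self.
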(event Custom|End_EnableCombo
  ;[1 1 1] Enable Combo
  (Variables|Default|SetEnable false))

(event Custom|Begin_EnableCombo
  ;[1 1 1] Enable Combo
  (Variables|Default|SetEnable true))

(event EventDoAction
  (bind _ownercharacter (Variables|Default|GetOwnerCharacter))
  ;[1 1 1] Do Action
  (|CallParentFunction)
  (if (CallFunction|IsExistAction)
    (if (Variables|Default|GetEnable)
      (Variables|Default|SetEnable false)
      (Variables|Default|SetExist true)
      (elif (Utilities|DoesObjectImplementInterface _ownercharacter "/Game/Interfaces/IState.IState_C")
        (bind _result (Class|IState|IsStateIdle(Message) _ownercharacter))
        (if _result
          (Class|IState|SetStateDoAction(Message) _ownercharacter)
          (CallFunction|PlayAction (Variables|Default|GetIndex)))))))

(event EventBeginDoAction
  ;[1 1 1] Begin Do Action
  (|CallParentFunction)
  (if (Variables|Default|GetExist)
    (Variables|Default|SetExist false)
    (Animation|StopAnimMontage (Variables|Default|GetOwnerCharacter) 0)
    (Math|Integer|IncrementInt (Variables|Default|GetIndex)
      (:%20%20
        (CallFunction|PlayAction (Variables|Default|GetIndex))))))

(event EventEndDoAction
  (bind _ownercharacter (Variables|Default|GetOwnerCharacter))
  ;[1 1 1] End Action
  (|CallParentFunction)
  (Variables|Default|SetIndex 0)
  (Animation|StopAnimMontage _ownercharacter 0)
  (if (Utilities|DoesObjectImplementInterface _ownercharacter "/Game/Interfaces/IState.IState_C")
    (Class|IState|SetStateIdle(Message) _ownercharacter)
    (if (Utilities|DoesObjectImplementInterface _ownercharacter "/Game/Interfaces/IWeapon.IWeapon_C")
      (Class|IWeapon|SetWeaponMove(Message) _ownercharacter))))

(event EventBeginPlay
  (|CallParentFunction)
  (Collision|RegistBeginOverlap)
  (Collision|OffCollsion))

(fn ConstructionScript
  (|CallParentFunction))

(fn BeginEquip
  (|CallParentFunction))

(fn RegistBeginOverlap
  (for _array_element (Actor|GetComponentsByClass "/Script/Engine.ShapeComponent")
    (Collision|BindEventtoOnComponentBeginOverlap _array_element (EventDispatchers|CreateEvent :!event OnBeginOverlap))))

(fn OnBeginOverlap
  (params (OverlappedComponent :type Primitive%20Component%20Object%20Reference) (OtherActor :type Actor%20Object%20Reference) (OtherComp :type Primitive%20Component%20Object%20Reference) (OtherBodyIndex :type Integer) (bFromSweep :type Boolean) (SweepResult :type Hit%20Result%20Structure%20%28by%20ref%29))
  (if (and (!= OtherActor (Variables|Default|GetOwnerCharacter)) (!= OtherActor self))
    (CallFunction|SendDamage OtherActor (CallFunction|GetAcitonDamage (Variables|Default|GetIndex)))))

(fn OnCollision
  (for _array_element (Actor|GetComponentsByClass "/Script/Engine.ShapeComponent")
    (Collision|SetCollisionEnabled _array_element "QueryAndPhysics")))

(fn OffCollsion
  (for _array_element (Actor|GetComponentsByClass "/Script/Engine.ShapeComponent")
    (Collision|SetCollisionEnabled _array_element "NoCollision")))