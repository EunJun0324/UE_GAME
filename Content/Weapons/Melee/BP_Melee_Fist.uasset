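; BP_Melee_Fist is a fist melee weapon that attaches itself to its owning character on BeginPlay, passing None as the attach name.
; It then moves each of its sphere components onto the owner's character mesh, using the component's object name as the socket name.
; Sphere names therefore choose which socket or bone each follows, while relative location, rotation and scale are kept.
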(event EventBeginPlay
  (|CallParentFunction)
  (CallFunction|AttachtoOwnerCharacter "None")
  (for _array_element (Actor|GetComponentsByClass "/Script/Engine.SphereComponent")
    (Transformation|AttachComponentToComponent _array_element (Variables|/Script/Engine.Character|GetMesh (Variables|Default|GetOwnerCharacter)) (Utilities|String|StringToName (Utilities|GetObjectName _array_element)) "KeepRelative" "KeepRelative" "KeepRelative" true)))

(fn ConstructionScript
  (|CallParentFunction))