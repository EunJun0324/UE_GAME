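; BP_FireStorm is a weapon action that sends a damaging fire storm circling around its owner.
; It starts only when the owner's IState reports idle, then attaches the effect to a collision box that Tick orbits around the owner from a random angle.
; Overlaps track characters other than the owner, and a looping timer damages them.
; Two seconds after the action ends, the effect, collision and timer are shut down.
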(event OnComponentBeginOverlap(Box)
  (params (OverlappedComponent :type Primitive%20Component%20Object%20Reference) (OtherActor :type Actor%20Object%20Reference) (OtherComp :type Primitive%20Component%20Object%20Reference) (OtherBodyIndex :type Integer) (bFromSweep :type Boolean) (SweepResult :type Hit%20Result%20Structure%20%28by%20ref%29))
  ;[1 1 1] OnComponetBeginOverlap
  (if (!= OtherActor (Variables|Default|GetOwnerCharacter))
    (bind _ascharacter (Utilities|Casting|CastToCharacter OtherActor))
    (Utilities|Array|AddUnique (Variables|Default|GetHitted) _ascharacter)))

(event OnComponentEndOverlap(Box)
  (params (OverlappedComponent :type Primitive%20Component%20Object%20Reference) (OtherActor :type Actor%20Object%20Reference) (OtherComp :type Primitive%20Component%20Object%20Reference) (OtherBodyIndex :type Integer))
  ;[1 1 1] OnComponentEndOverlap
  (for (_array_element _array_index) (Variables|Default|GetHitted)
    (if (== _array_element OtherActor)
      (Utilities|Array|RemoveIndex (Variables|Default|GetHitted) _array_index))))

(event Custom|OnHitTimer
  ;[1 1 1] OnHitTimer
  (for _array_element (Variables|Default|GetHitted)
    (CallFunction|SendDamage _array_element (CallFunction|GetActionDamage))))

(event EventBeginPlay
  ;[1 1 1] BeginPlay
  (|CallParentFunction)
  (Collision|SetCollisionEnabled (Variables|Default|GetBox) "NoCollision"))

(event EventDoAction
  (bind _ownercharacter (Variables|Default|GetOwnerCharacter))
  ;[1 1 1] DoAction
  (|CallParentFunction)
  (if (Utilities|DoesObjectImplementInterface _ownercharacter "/Game/Interfaces/IState.IState_C")
    (bind _result (Class|IState|IsStateIdle(Message) _ownercharacter))
    (if _result
      (Class|IState|SetStateDoAction(Message) _ownercharacter)
      (CallFunction|PlayAction))))

(event EventBeginDoAction
  (bind (_effect _effectlocation _effectscale _effectrotation) (CallFunction|GetActionEffect))
  (bind _ownercharacter (Variables|Default|GetOwnerCharacter))
  ;[1 1 1] BeginDoAction
  (|CallParentFunction)
  (bind _returnvalue (Effects|SpawnEmitterAttached _effect (Variables|Default|GetBox) "None" _effectlocation _effectrotation _effectscale))
  (Variables|컴포넌트|SetParticle _returnvalue)
  (Variables|Default|SetAngle (Math|Random|RandomFloatinRange 0.0 3.6e+02))
  (Collision|SetCollisionEnabled (Variables|Default|GetBox) "QueryAndPhysics")
  (Utilities|Time|SetTimerbyFunctionName self "OnHitTimer" (Variables|Default|GetHitTimer) true)
  (if (Utilities|DoesObjectImplementInterface _ownercharacter "/Game/Interfaces/IState.IState_C")
    (Class|IState|SetStateIdle(Message) _ownercharacter)))

(event EventEndDoAction
  ;[1 1 1] EndDoAction
  (|CallParentFunction)
  (Utilities|FlowControl|Delay 2.0)
  (Components|DestroyComponent (Variables|컴포넌트|GetParticle))
  (Collision|SetCollisionEnabled (Variables|Default|GetBox) "NoCollision")
  (Utilities|Time|ClearTimerbyFunctionName self "OnHitTimer"))

(event EventTick
  (params (DeltaSeconds :type Float%20%28single-precision%29))
  ;[1 1 1] Tick
  (Variables|컴포넌트|GetParticle
    (:then
      (Utilities|FlowControl|Sequence
        (:then_0
          (bind _output_get (Variables|Default|SetAngle (+ (* (Variables|Default|GetSpeed) (Utilities|Time|GetWorldDeltaSeconds)) (Variables|Default|GetAngle))))
          (if (Math|Float|NearlyEqual(Float) _output_get 3.6e+02 1e-06)
            (Variables|Default|SetAngle 0.0)))
        (:then_1
          (Transformation|SetWorldLocation (Variables|Default|GetBox) (+ (Math|Vector|RotateVectorAroundAxis "250.000000, 0, 0" (Variables|Default|GetAngle) "0, 0,1.000000") (Transformation|GetActorLocation (Variables|Default|GetOwnerCharacter))) false false))))
    (:else)))

(fn ConstructionScript
  (|CallParentFunction))