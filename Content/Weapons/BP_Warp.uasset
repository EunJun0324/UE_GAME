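; BP_Warp is an equippable item that teleports its owner to the point under the cursor.
; While equipped by an owner tagged Player, Tick projects a decal onto WorldStatic cursor hits, aligned to the surface normal.
; DoAction caches the hit and, if the owner's IState is idle, sets the action state and plays the action.
; BeginDoAction attaches an effect, then EndDoAction moves the owner there and restores idle.
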(event EventBeginPlay
  ;[1 1 1] BeginPlay
  (|CallParentFunction)
  (Rendering|SetVisibility (Variables|Default|GetDecal) false false))

(event EventTick
  (params (DeltaSeconds :type Float%20%28single-precision%29))
  (bind (_hitresult _hitresultimpactpoint _hitresultimpactnormal) (CallFunction|GetCursorLocationandRataion))
  (bind _decal (Variables|Default|GetDecal))
  ;[1 1 1] Tick
  (if (CallFunction|GetEqquiped)
    (if (CallFunction|IsVisibleCursor)
      (if _hitresult
        (Rendering|SetVisibility _decal true false)
        (Transformation|SetWorldLocationAndRotation (Variables|Default|GetDecal) _hitresultimpactpoint _hitresultimpactnormal false false)
        (else
          (Rendering|SetVisibility _decal false false :!label _label)))
      (else
        (goto _label)))))

(event EventDoAction
  (bind (_hitresult _hitresultimpactpoint) (CallFunction|GetCursorLocationandRataion))
  (bind _ownercharacter (Variables|Default|GetOwnerCharacter))
  ;[1 1 1] DoAction
  (|CallParentFunction)
  (if (CallFunction|IsVisibleCursor)
    (Variables|Default|SetPossible _hitresult)
    (Variables|Default|SetImpointPoint _hitresultimpactpoint)
    (if _hitresult
      (if (Utilities|DoesObjectImplementInterface _ownercharacter "/Game/Interfaces/IState.IState_C")
        (bind _result (Class|IState|IsStateIdle(Message) _ownercharacter))
        (if _result
          (Class|IState|SetStateDoAction(Message) _ownercharacter)
          (CallFunction|PlayAction))))))

(event EventBeginDoAction
  (bind (_effect _effectlocation _effectscale _effectrotation) (CallFunction|GetActionEffect))
  ;[1 1 1] Begin Do Action
  (|CallParentFunction)
  (if (Variables|Default|GetPossible)
    (Effects|SpawnEmitterAttached _effect (Variables|/Script/Engine.Character|GetMesh (Variables|Default|GetOwnerCharacter)) "None" _effectlocation _effectrotation _effectscale)))

(event EventEndDoAction
  (bind _ownercharacter (Variables|Default|GetOwnerCharacter))
  ;[1 1 1] EndDoAction
  (|CallParentFunction)
  (if (Variables|Default|GetPossible)
    (Transformation|SetActorLocation _ownercharacter (Variables|Default|GetImpointPoint) false false)
    (Class|IState|SetStateIdle(Message) _ownercharacter)))

(event EventUnequip
  ;[1 1 1] Unequip
  (|CallParentFunction)
  (Rendering|SetVisibility (Variables|Default|GetDecal) false false))

(fn ConstructionScript
  (|CallParentFunction))

(fn IsVisibleCursor
  (for _array_element (Variables|/Script/Engine.Actor|GetTags (Variables|Default|GetOwnerCharacter))
    (if (Utilities|Name|Equal(Name) _array_element (Utilities|Name|MakeLiteralName "Player"))
      (return true)))
  (return false))

(fn GetCursorLocationandRataion
  (bind _returnvalue (Game|GetPlayerController 0))
  (bind _array (Utilities|Array|MakeArray "ObjectTypeQuery1"))
  (bind (_hitresult _returnvalue_2) (Class|PlayerController|GetHitResultUnderCursorforObjects _returnvalue _array false))
  (return _returnvalue_2 (.impactpoint _hitresult) (Math|Conversions|RotationFromXVector (.impactnormal _hitresult))))