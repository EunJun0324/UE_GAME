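; BP_FireBall is a fireball weapon Blueprint that extends a parent class's equip lifecycle with a visible particle effect.
; On BeginPlay it runs the parent logic, attaches to the owner character with no named socket, and hides its ParticleSystem.
; The effect appears when EndEquip fires and hides again on Unequip, with both events calling their parent versions first.
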(event EventBeginPlay
  ;[1 1 1] Begin Play
  (|CallParentFunction)
  (CallFunction|AttachtoOwnerCharacter "None")
  (Rendering|SetVisibility (Variables|Default|GetParticleSystem) false false))

(event EventEndEquip
  ;[1 1 1] EndEquip
  (|CallParentFunction)
  (Rendering|SetVisibility (Variables|Default|GetParticleSystem) true false))

(event EventUnequip
  ;[1 1 1] UnEquip
  (|CallParentFunction)
  (Rendering|SetVisibility (Variables|Default|GetParticleSystem) false false))

(fn ConstructionScript
  (|CallParentFunction))